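; BP_Doors_01 is an architectural visualisation door built from frame, leaf and handle static meshes, configurable to AU, EU or US standard sizes.
; GetDoorID maps the size enum to a structure entry, supplying frame and door meshes plus offsets to the construction script.
; The script positions and rotates the parts, mirroring the frame's Y scale for left hinges; size-based scaling is disconnected.
; SetMaterialsByID applies colour-scheme materials but is not called here.
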(fn `GetDoorID`
  (returns (DoorValues :type "/Game/ArchVizUI_V3/Assets/Building/Doors/BPS_DoorSizes Structure") (ID :type Integer))
  (bind _returnvalue (select `/Game/ArchVizUI_V3/Assets/Building/Doors/Enum_DoorSizes` (`self.DoorSizes`) :`NewEnumerator2` 1 :`NewEnumerator9` 2 :`NewEnumerator13` 3 :`NewEnumerator15` 4 :`NewEnumerator14` 5 :`NewEnumerator0` 6 :`NewEnumerator16` 7 :`NewEnumerator17` 8 :`NewEnumerator18` 9 :`NewEnumerator19` 10 :`NewEnumerator20` 11 :`NewEnumerator1` 12 :`NewEnumerator6` 13 :`NewEnumerator7` 14 :`NewEnumerator11` 15 :`NewEnumerator8` 16 :`NewEnumerator10` 17 :`NewEnumerator21` 18 :`NewEnumerator22` 19 :`NewEnumerator23` 20))
  (return (`|GetArrayItem` (`self.DoorSizesStructure`) _returnvalue) _returnvalue))

(fn `SetMaterialsByID`
  (params (Materials :type "Array of /Game/ArchVizUI_V3/Assets/Building/Doors/BPS_MatWithID Structure") (Mesh :type "StaticMeshComponent Object Reference") (ColourSchemeID :type Integer))
  (for _array_element Materials
    (bind (_material _matid _colorschemeid) (break `/Game/ArchVizUI_V3/Assets/Building/Doors/BPS_MatWithID` _array_element))
    (if (== _colorschemeid ColourSchemeID)
      (`PrimitiveComponent.SetMaterial` Mesh _matid _material))))

(fn `UserConstructionScript`
  (locals (NewLocalVar_0 :type "Rotator Structure" :default (struct)))
  (bind (_doorrelativelocation_x _doorrelativelocation_y _doorrelativelocation_z) (`KismetMathLibrary.BreakVector` (`self.DoorRelativeLocation`)))
  (bind (_doorrelativelocation_x_2 _doorrelativelocation_y_2 _doorrelativelocation_z_2) (`KismetMathLibrary.BreakVector` (`self.DoorRelativeLocation`)))
  (`|ExecutionSequence`
    (:`then_1`
      ;[1 1 1] set frame
      (`StaticMeshComponent.SetStaticMesh` (`self.DoorFrame`) (select `bool` false :`false` (`.Frame_23_BBD341C547B9886A39E8B986AB536363` (break `/Game/ArchVizUI_V3/Assets/Building/Doors/BPS_DoorSizes` (`self.GetDoorID`))) :`true` (`self.FrameMesh`)))
      ;[1 1 1] set door
      (`StaticMeshComponent.SetStaticMesh` (select `bool` false :`false` (`self.DoorStatic`)) (select `bool` false :`false` (`.Door_24_F6E5DFE142EEBA190E053BB6B170DC7B` (break `/Game/ArchVizUI_V3/Assets/Building/Doors/BPS_DoorSizes` (`self.GetDoorID`))) :`true` (`self.DoorMesh`)))
      ;[1 1 1] set handle
      (`StaticMeshComponent.SetStaticMesh` (select `bool` false :`false` (`self.HandleStatic`)) (`self.HandleMesh`)))
    (:`then_2`
      ;[1 1 1] offset scale rotation
      (`SceneComponent.K2_AddLocalOffset` (`self.DoorStatic`) (`KismetMathLibrary.MakeVector` _doorrelativelocation_x_2 (`.DoorOffset_14_E79C5ED340E0A2DA9FC3FAA49316DA99` (break `/Game/ArchVizUI_V3/Assets/Building/Doors/BPS_DoorSizes` (`self.GetDoorID`))) _doorrelativelocation_z_2) false false)
      (`SceneComponent.K2_AddLocalOffset` (`self.HandleStatic`) (`KismetMathLibrary.MakeVector` _doorrelativelocation_x (`.HandleOffset_16_C5AADC13411CB189712691A4FBA1CDA5` (break `/Game/ArchVizUI_V3/Assets/Building/Doors/BPS_DoorSizes` (`self.GetDoorID`))) _doorrelativelocation_z) false false)
      (`SceneComponent.K2_SetRelativeRotation` (`self.DoorStatic`) (`KismetMathLibrary.MakeRotator` 0.0 0.0 (* (`self.DoorRotation`) -1.0)) false false)
      (if (not (`self.HingeOnRight`))
        (`SceneComponent.SetRelativeScale3D` (`self.DoorFrame`) (1.0 -1.0 1.0))))))